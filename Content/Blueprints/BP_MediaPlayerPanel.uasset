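; BP_MediaPlayerPanel is an actor that plays a video file on a plane in the level.
; On BeginPlay, LoadFile opens FilePath in the media player, links the media texture and starts playback.
; It then applies a dynamic material instance to the plane with that texture as its Texture parameter.
; OpenFilePathWidget can show a file-picker widget holding a back-reference to the panel, but it is never called here, and the ShouldOpenWidget branch is empty.
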(event `self.ReceiveBeginPlay`
  (`self.LoadFile`)
  (if (`self.bShouldOpenWidget`)
    _))

(fn `LoadFile`
  (bind _mediaplayer (`self.MediaPlayer`))
  (bind _mediatexture (`self.MediaTexture`))
  (`MediaPlayer.OpenFile` _mediaplayer (`self.FilePath`))
  (`MediaTexture.SetMediaPlayer` _mediatexture _mediaplayer)
  (`MediaPlayer.Play` _mediaplayer)
  (bind _returnvalue (`PrimitiveComponent.CreateDynamicMaterialInstance` (`self.Plane`) 0 (`self.Material`) "None"))
  (`MaterialInstanceDynamic.SetTextureParameterValue` _returnvalue "Texture" _mediatexture))

(fn `OpenFilePathWidget`
  (bind _returnvalue (`|CreateWidget` "/VideoCheckers3DPlayer/Widgets/OpenVideoFileWidget.OpenVideoFileWidget_C" (`GameplayStatics.GetPlayerController` 0)))
  (set `self.FilePathWidget` _returnvalue)
  (set `/VideoCheckers3DPlayer/Widgets/OpenVideoFileWidget.Media Player` self (`self.FilePathWidget`))
  (`UserWidget.AddToViewport` _returnvalue 0))

(fn `UserConstructionScript`)